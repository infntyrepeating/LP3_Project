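; BP_NavMoving is an actor that slides back and forth along Y from its starting position, like a moving wall.
; After a short delay on BeginPlay, it stores no further input and runs MovingAction, driving the WallMovement timeline forward or in reverse based on the DoStart flag.
; Timeline updates offset the relative location, and each finish flips the flag, pauses, then calls MovingAction again for an endless loop.
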(event `self.ReceiveBeginPlay`
  (set `self.doStart` true)
  (set `self.InitialLoc` (`self.GetTransform`))
  (`KismetSystemLibrary.Delay` 2.0)
  (`self.MovingAction`))

(event `MovingAction`
  (if (`self.doStart`)
    (bind (_direction _floatmovement) (`Timeline|WallMovement` :!via `PlayFromStart` :!label _label)
      (:`Update`
        (`self.K2_SetActorRelativeLocation` (`KismetMathLibrary.MakeVector` (.x (.location (`self.InitialLoc`))) (+ _floatmovement (.y (.location (`self.InitialLoc`)))) (.z (.location (`self.InitialLoc`))))))
      (:`Finished`
        (set `self.doStart` (not (`self.doStart`)))
        (`KismetSystemLibrary.Delay` 5.0)
        (`self.MovingAction`)))
    (else
      (goto _label :!via `ReverseFromEnd`))))

(fn `UserConstructionScript`)