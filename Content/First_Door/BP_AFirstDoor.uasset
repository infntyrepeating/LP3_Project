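; BP_AFirstDoor is a door actor that toggles between open and closed on interaction.
; OnInteract plays the DoorAnimation timeline forward or reverses it from the end, based on IsDoorOpen.
; The timeline's Opening track drives the relative yaw of the Arrow component.
; An AnimationOnGoing flag ignores interaction during the swing, and completion flips the open state and releases the lock.
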(event `self.ReceiveBeginPlay`
  (set `self.isDoorOpen` false))

(event `/Game/First_Door/IF_InteractableFD.OnInteract`
  (if (not (`self.animationOnGoing`))
    (set `self.animationOnGoing` true)
    (if (`self.isDoorOpen`)
      (bind (_direction _opening) (`Timeline|DoorAnimation` :!via `ReverseFromEnd` :!label _label)
        (:`Update`
          (`SceneComponent.K2_SetRelativeRotation` (`self.Arrow`) (`KismetMathLibrary.MakeRotator` 0.0 0.0 _opening) false false))
        (:`Finished`
          (set `self.isDoorOpen` (not (`self.isDoorOpen`)))
          (set `self.animationOnGoing` false)))
      (else
        (goto _label)))))

(fn `UserConstructionScript`)