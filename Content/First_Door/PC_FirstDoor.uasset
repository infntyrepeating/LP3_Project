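; Player controller for the First Door area that turns input into pawn movement and interaction.
; Forward and sideways axes add movement input along fixed world directions, derived from a zero rotation and a 90-degree offset, independent of camera or pawn facing.
; The interaction key casts the controlled pawn to BP_CFirstDoor and passes the press on to that character's handler.
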(event `InputAxis|ForwardAxis`
  (params (AxisValue :type "Float (single-precision)"))
  (`Pawn.AddMovementInput` (`self.K2_GetPawn`) (`KismetMathLibrary.GetForwardVector` (struct)) AxisValue false))

(event `InputAxis|SidewaysAxis`
  (params (AxisValue :type "Float (single-precision)"))
  (`Pawn.AddMovementInput` (`self.K2_GetPawn`) (`KismetMathLibrary.GreaterGreater_VectorRotator` (`KismetMathLibrary.GetForwardVector` (struct)) (struct :`Yaw` 90.0)) AxisValue false))

(event `InputAction|InteractionKey`
  (params (Key :type "Key Structure"))
  (:`Pressed`
    (bind _asbp_cfirst_door (cast `/Game/First_Door/BP_CFirstDoor` (`self.K2_GetPawn`)))
    (`/Game/First_Door/BP_CFirstDoor.InteractionKeyPressed` _asbp_cfirst_door)))

(fn `UserConstructionScript`)