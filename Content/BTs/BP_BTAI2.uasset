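; BP_BTAI2 is an AI controller that runs the AI_Second behavior tree and tracks the player by sight.
; Perception updates feed SightHandler, which ignores non-sight stimuli and actors other than the player.
; It sets TargettedActor to the player when seen or clears it when lost, writing the stimulus location to lastKnownLoc either way.
; GetStart exposes the controlled BP_AI2 pawn's starting location.
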(event `self.ReceiveBeginPlay`
  (`self.RunBehaviorTree` "/Game/BTs/AI_Second.AI_Second"))

(event `self.AIPerception.OnTargetPerceptionUpdated`
  (params (Actor :type "Actor Object Reference") (Stimulus :type "AIStimulus Structure"))
  (`self.Sight Handler` Actor Stimulus))

(fn `Get Start`
  (returns (NewParam :type "Vector Structure"))
  (bind _asbp_ai2 (cast `/Game/BTs/BP_AI2` (`self.K2_GetPawn`)))
  (return (`/Game/BTs/BP_AI2.StartingLoc` _asbp_ai2)))

(fn `Sight Handler`
  (params (Actor :type "Actor Object Reference") (Stimulus :type "AIStimulus Structure"))
  (bind (_stimulus_age _stimulus_expirationage _stimulus_strength _stimulus_stimuluslocation _stimulus_receiverlocation _stimulus_tag _stimulus_bsuccessfullysensed) (break `AIStimulus` (`local.Stimulus`)))
  (bind _returnvalue (`AIPerceptionSystem.GetSenseClassForStimulus` Stimulus))
  (if (== _returnvalue "/Script/AIModule.AISense_Sight")
    (if (== (`local.Actor`) (`GameplayStatics.GetPlayerCharacter` 0))
      (`BlackboardComponent.SetValueAsObject` (`self.Blackboard`) "TargettedActor" (`KismetMathLibrary.SelectObject` (`GameplayStatics.GetPlayerCharacter` 0) null _stimulus_bsuccessfullysensed))
      (`BlackboardComponent.SetValueAsVector` (`self.Blackboard`) "lastKnownLoc" _stimulus_stimuluslocation)
      (else
        (return)))
    (else
      (return))))

(fn `UserConstructionScript`)