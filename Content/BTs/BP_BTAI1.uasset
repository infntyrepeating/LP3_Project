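; BP_BTAI1 is an AI controller that runs the AI_First behavior tree on BeginPlay and feeds it sightings of the player.
; Perception updates go to SightHandler, which ignores everything except sight stimuli from player character 0.
; It sets TargetActor to the player when sensed and clears it when sight is lost.
; Either update also stores the stimulus location as lastKnownLocation and resets the TriesLeft counter.
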(event `self.ReceiveBeginPlay`
  (`self.RunBehaviorTree` "/Game/BTs/AI_First.AI_First"))

(event `self.AIPerception.OnTargetPerceptionUpdated`
  (params (Actor :type "Actor Object Reference") (Stimulus :type "AIStimulus Structure"))
  (`self.Sight Handler` Actor Stimulus))

(fn `Sight Handler`
  (params (Actor :type "Actor Object Reference") (Stimulus :type "AIStimulus Structure"))
  (bind _blackboard (`self.Blackboard`))
  (bind (_stimulus_age _stimulus_expirationage _stimulus_strength _stimulus_stimuluslocation _stimulus_receiverlocation _stimulus_tag _stimulus_bsuccessfullysensed) (break `AIStimulus` (`local.Stimulus`)))
  (bind _returnvalue (`AIPerceptionSystem.GetSenseClassForStimulus` Stimulus))
  (if (== _returnvalue "/Script/AIModule.AISense_Sight")
    (if (== (`local.Actor`) (`GameplayStatics.GetPlayerCharacter` 0))
      (`BlackboardComponent.SetValueAsObject` (`self.Blackboard`) "TargetActor" (`KismetMathLibrary.SelectObject` (`GameplayStatics.GetPlayerCharacter` 0) null _stimulus_bsuccessfullysensed))
      (`BlackboardComponent.SetValueAsVector` _blackboard "lastKnownLocation" _stimulus_stimuluslocation)
      (`BlackboardComponent.SetValueAsInt` _blackboard "TriesLeft" 6)
      (else
        (return)))
    (else
      (return))))

(fn `UserConstructionScript`)